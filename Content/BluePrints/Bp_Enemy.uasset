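; Enemy Blueprint that destroys itself when its health drops below zero, including on contact with the first-person player.
; From BeginPlay, a CheckHealth event re-calls itself after a short delay to poll Health, rather than reacting to changes.
; A capsule overlap with BP_FirstPersonCharacter sets Health negative, so the next poll destroys the enemy.
; Zero health still counts as alive.
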(event `self.ReceiveBeginPlay`
  (`self.Check Health`))

(event `Check Health`
  (`KismetSystemLibrary.Delay` 0.2)
  (if (>= (`self.health`) 0.0)
    (`self.Check Health`)
    (else
      (`self.K2_DestroyActor`))))

(event `self.Capsule Collision.OnComponentBeginOverlap`
  (params (OverlappedComponent :type "PrimitiveComponent Object Reference") (OtherActor :type "Actor Object Reference") (OtherComp :type "PrimitiveComponent Object Reference") (OtherBodyIndex :type Integer) (bFromSweep :type Boolean) (SweepResult :type "HitResult Structure (by ref)"))
  (cast `/Game/FirstPerson/Blueprints/BP_FirstPersonCharacter` OtherActor)
  (set `self.health` -1.0))

(fn `UserConstructionScript`)