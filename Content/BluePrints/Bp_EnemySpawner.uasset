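; Enemy spawner Blueprint that fills the level with enemies in waves, respawning whenever none are left.
; On BeginPlay it gathers all Bp_EnemySpawnLocation actors, prints their count, then spawns a Bp_Enemy at each with a high random probability.
; A self-calling, delayed check loop polls every couple of seconds with the costly GetAllActorsOfClass and triggers a new wave when no Bp_Enemy remains.
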(event `self.ReceiveBeginPlay`
  (bind _outactors (`GameplayStatics.GetAllActorsOfClass` "/Game/BluePrints/Bp_EnemySpawnLocation.Bp_EnemySpawnLocation_C"))
  (`KismetSystemLibrary.PrintString` (`KismetStringLibrary.Concat_StrStr` "there are " (`KismetStringLibrary.Conv_IntToString` (`KismetArrayLibrary.Array_Length` _outactors)) " spawn locations.") true true (struct :`G` 0.66 :`B` 1.0 :`A` 1.0) 10.0)
  (`self.Spawn Enemies`)
  (`self.check enemy count`))

(event `Spawn Enemies`
  (for _array_element (stale `self.ReceiveBeginPlay` _outactors)
    (if (< (`KismetMathLibrary.RandomFloat`) 0.8)
      ;[1 1 1] Spawn actor from class
      (`|SpawnActorFromClass` "/Game/BluePrints/Bp_Enemy.Bp_Enemy_C" (`self.GetTransform` _array_element) "Undefined" "MultiplyWithRoot" null null))))

(event `check enemy count`
  ;[1 1 1] This is the expensive one
  (bind _outactors (`GameplayStatics.GetAllActorsOfClass` "/Game/BluePrints/Bp_Enemy.Bp_Enemy_C"))
  (if (not (> (`KismetArrayLibrary.Array_Length` _outactors) 0))
    (`self.Spawn Enemies`))
  (`KismetSystemLibrary.Delay` 2.0)
  (`self.check enemy count`))

(fn `UserConstructionScript`)